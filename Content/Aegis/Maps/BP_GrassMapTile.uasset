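; BP_GrassMapTile is a grass map tile that can switch to a debug view of its pathing gradient.
; On BeginPlay it applies a new dynamic material instance to TileMesh: M_DebugGradient fed PathingGradient as a scalar when IsShowingGradients is set, otherwise M_GrassTile.
; ToggleShowGradients flips that flag and reruns the same material logic, creating a fresh instance each time.
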(event `self.ReceiveBeginPlay`
  (bind _tilemesh (`self.TileMesh`))
  (if (stale `self.ToggleShowGradients` _output_get) :!label _label
    (bind _returnvalue (`KismetMaterialLibrary.CreateDynamicMaterialInstance` "/Game/Aegis/Maps/M_DebugGradient.M_DebugGradient"))
    (`MaterialInstanceDynamic.SetScalarParameterValue` _returnvalue "Gradient" (`self.PathingGradient`))
    (`PrimitiveComponent.SetMaterial` _tilemesh 0 _returnvalue)
    (else
      (bind _returnvalue_2 (`KismetMaterialLibrary.CreateDynamicMaterialInstance` "/Game/Aegis/Maps/M_GrassTile.M_GrassTile"))
      (`PrimitiveComponent.SetMaterial` _tilemesh 0 _returnvalue_2))))

(event `self.ToggleShowGradients`
  (bind _output_get (set `self.IsShowingGradients` (not (`self.IsShowingGradients`))))
  (goto _label))

(fn `UserConstructionScript`)