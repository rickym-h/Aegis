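; BP_TestEnemy is a test enemy drawn with a flipbook sprite and carrying a widget health bar.
; BeginPlay caches the WBP_EnemyHPBar widget, then sets fixed tilted rotations once on the bar and sprite, taking only the bar's roll from a look-at toward the player camera.
; Tick copies the enemy's health percentage into the cached bar every frame.
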(event `self.ReceiveBeginPlay`
  (bind _aswbp_enemy_hpbar (cast `/Game/Aegis/Widgets/GamePlayUI/WBP_EnemyHPBar` (`WidgetComponent.GetWidget` (`self.Widget`))))
  (set `self.As WBP Enemy HPBar` _aswbp_enemy_hpbar)
  (`SceneComponent.K2_SetWorldRotation` (`self.Widget`) (`KismetMathLibrary.MakeRotator` (.roll (`KismetMathLibrary.FindLookAtRotation` (`SceneComponent.K2_GetComponentLocation` (`self.RootComponent`)) (`SceneComponent.K2_GetComponentLocation` (`PlayerCameraManager.TransformComponent` (`GameplayStatics.GetPlayerCameraManager` 0))))) 0.0 180.0) false false)
  (`SceneComponent.K2_SetWorldRotation` (`self.FlipbookComponent`) (`KismetMathLibrary.MakeRotator` -30.0 0.0 90.0) false false))

(event `self.ReceiveTick`
  (params (DeltaSeconds :type "Float (single-precision)"))
  (set `/Game/Aegis/Widgets/GamePlayUI/WBP_EnemyHPBar.HealthAsPercentage` (`self.GetHealthAsPercentage`) (`self.As WBP Enemy HPBar`)))

(fn `UserConstructionScript`)